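; Player hero pawn with cursor aiming, axis movement, Shift-held camera rotation and item pickup on overlap.
; Primary and secondary fire route through ShootServerSide to replicated shot and capacity events, which are empty here.
; Movement is relayed manually: MoveCtoS stores transforms in gs_Main, then MoveStoC applies them to non-local copies.
; Tick updates aim, turns the actor toward velocity, and applies custom gravity from a downward ground trace.
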(event OnComponentBeginOverlap(Projectilecollider)
  (params (OverlappedComponent :type Primitive%20Component%20Object%20Reference) (OtherActor :type Actor%20Object%20Reference) (OtherComp :type Primitive%20Component%20Object%20Reference) (OtherBodyIndex :type Integer) (bFromSweep :type Boolean) (SweepResult :type Hit%20Result%20Structure%20%28by%20ref%29))
  (bind _asbp_item_parent (Utilities|Casting|CastTobp_ItemParent OtherActor))
  (bind _aspc_main (Utilities|Casting|CastTopc_Main (Pawn|GetController)))
  (bind (_succes_ _rest) (Default|AddItem _aspc_main (Utilities|GetClass _asbp_item_parent) (Variables|/Game/Blueprints/Inventory/Items/bp_ItemParent.bp_ItemParent_C|GetAmount _asbp_item_parent)))
  (if _succes_
    (if (> _rest 0)
      (Variables|/Game/Blueprints/Inventory/Items/bp_ItemParent.bp_ItemParent_C|SetAmount _asbp_item_parent 0)
      (else
        (Actor|DestroyActor OtherActor)))))

(event Custom|Secondary%20Shoot
  ;[1 0.9375 0 0.5] Fire System
  ;;[1 0 0 0.5] Send Basefire info to serv
  (Variables|Default|SetShootType "NewEnumerator1")
  (bind _aspc_main (Utilities|Casting|CastTopc_Main (Pawn|GetController)))
  (CallFunction|ShootServerSide (Variables|Default|GetShootType) (Variables|GetPlayerState) (+ (* (Math|Vector|GetForwardVector (Variables|Default|GetCursor%20Direction)) 20) (Transformation|GetWorldLocation (Variables|Default|Getarrow_forward))) (Variables|Default|GetCursor%20Direction) _aspc_main))

(event Custom|Actor%20Face%20velocity%20Vector
  (bind _returnvalue (Transformation|GetActorRotation))
  (bind _floatingpawnmovement (Variables|Default|GetFloatingPawnMovement))
  (bind (_roll _pitch) (Math|Rotator|BreakRotator _returnvalue))
  (bind _velocity (Variables|/Script/Engine.MovementComponent|GetVelocity _floatingpawnmovement))
  ;[0 0.5547 1 0.5] Local focus
  ;;[0.8984 0 1 0.5] Actor Face velocity Vector
  (Transformation|SetActorRotation (Math|Rotator|Lerp(Rotator) _returnvalue (select (Math|Vector|Equal(Vector) _velocity "0, 0, 0" 0.0001) _returnvalue (Math|Rotator|MakeRotator _roll _pitch (+ (.Yaw (Math|Rotator|BreakRotator (Math|Rotator|MakeRotfromZ _velocity))) -9e+01))) (* 20 (Utilities|Time|GetWorldDeltaSeconds)) true)))

(event Custom|PrimaryShoot%20server%20replicated%20to%20client
  (params (Start%20Location :type Vector) (Projectile%20Rotation :type Rotator) (Player%20Tag :type Name))
  ;[1 0.9375 0 0.5] Fire System
  ;;[0.1484 0 1 0.5] PrimaryShootserver replicated to client (one bullet)
)

(event Custom|Camera%20orientaiton%20Start
  ;[0.4531 0 1 0.5] Camera system
  ;;[1 0 0.2109 0.5] Camera orientation Start
  (Pawn|Input|AddControllerYawInput -2e+01))

(event Custom|Squeeze%20when%20shoot
  ;[1 0.9375 0 0.5] Fire System
  ;;[0.2422 1 0 0.5] Squeeze when shoot
  (bind _newtrack_1 (Timeline|ShootSqueeze PlayFromStart)
    (:Update
      (Transformation|SetWorldScale3D (Variables|Default|GetSkeletalMesh) _newtrack_1))))

(event Custom|Move%20CtoS
  (params (NewParam :type Pc%20Main%20Object%20Reference) (NewLocation :type Vector) (NewRotation :type Rotator))
  ;[1 0.9375 0 0.5] Mouvement
  ;;[0.8281 0 1 0.5] Movement CtoS
  (bind _asgs_main (Utilities|Casting|CastTogs_Main (Game|GetGameState)))
  (Default|StockPlayerPosition _asgs_main NewParam (Math|Transform|MakeTransform NewLocation NewRotation))
  (CallFunction|MoveStoC NewLocation NewRotation))

(event Custom|Move%20StoC
  (params (NewLocation :type Vector) (NewRotation :type Rotator))
  ;[1 0.9375 0 0.5] Mouvement
  ;;[0 1 0.3672 0.5] Movement StoC
  (if (not (Pawn|IsLocallyControlled))
    (Transformation|SetActorLocationAndRotation NewLocation NewRotation)))

(event Custom|Shoot%20ServerSide
  (params (Selection :type e_ShootType%20Enum :default "NewEnumerator0") (PlayerState :type Player%20State%20Object%20Reference) (Start%20location :type Vector) (Rotation%20of%20shooter :type Rotator) (Pc%20of%20shooter :type Pc%20Main%20Object%20Reference))
  ;[1 0.9375 0 0.5] Fire System
  ;;[0.9688 0 1 0.5] Analyse info of player and call Primary/Secondary to clients
  (Utilities|Casting|CastTops_Main PlayerState)
  (switch Utilities|FlowControl|Switch|Switchone_ShootType Selection
    (:NewEnumerator0
      (CallFunction|PrimaryShootServerReplicatedtoClient Start%20location Rotation%20of%20shooter (Utilities|Struct|Breaks_PlayerInfos (Variables|/Game/Blueprints/Player/pc_Main.pc_Main_C|GetPlayerInfos Pc%20of%20shooter))))
    (:NewEnumerator1
      (CallFunction|CapacityServerReplicatedtoClient))))

(event Custom|Capacity%20server%20replicated%20to%20client
  ;[1 0.9375 0 0.5] Fire System
  ;;[1 0 0.2344 0.5] Capacity server replicated to client
)

(event Custom|Mesh%20look%20cursor
  (bind _returnvalue (Pawn|GetController))
  (bind _aspc_main (Utilities|Casting|CastTopc_Main _returnvalue))
  (bind _hit_worldcursor (Variables|/Game/Blueprints/Player/pc_Main.pc_Main_C|Gethit_WorldCursor _aspc_main))
  ;[0 0.5547 1 0.5] Local focus
  ;;[0.7812 1 0 0.5] Mesh look cursor
  (if (Pawn|IsLocallyControlled)
    (if (.bblockinghit _hit_worldcursor)
      (Variables|Default|SetCursor%20Direction (Math|Rotator|MakeRotator 0.0 0.0 (+ (.Yaw (Math|Rotator|BreakRotator (Math|Rotator|MakeRotfromZ (* (Math|Vector|GetUnitDirection(Vector) (Transformation|GetWorldLocation (Variables|Default|GetCollider)) (.location _hit_worldcursor)) -1.0)))) 9e+01)))
      (else
        (Variables|Default|SetCursor%20Direction (Math|Rotator|MakeRotator 0.0 0.0 (+ (.Yaw (Math|Rotator|BreakRotator (Math|Rotator|MakeRotfromZ (* (Transformation|GetActorForwardVector) -1.0)))) 9e+01)) :!label _label)))
    (else
      (goto _label))))

(event Custom|Primary%20Shoot
  ;[1 0.9375 0 0.5] Fire System
  ;;[1 0 0 0.5] Send Basefire info to serv
  (Variables|Default|SetShootType "NewEnumerator0")
  (bind _aspc_main (Utilities|Casting|CastTopc_Main (Pawn|GetController)))
  (CallFunction|ShootServerSide (Variables|Default|GetShootType) (Variables|GetPlayerState) (+ (* (Math|Vector|GetForwardVector (Variables|Default|GetCursor%20Direction)) 20) (Transformation|GetWorldLocation (Variables|Default|Getarrow_forward))) (Variables|Default|GetCursor%20Direction) _aspc_main))

(event EventBeginPlay
  ;[1 0.75 0 0.5] Begin play
)

(event EventTick
  (params (DeltaSeconds :type Float%20%28single-precision%29))
  ;[0.8516 0 1 0.5] Tick
  (CallFunction|MeshLookCursor)
  (CallFunction|IsJumping?)
  (CallFunction|Gravity)
  (CallFunction|ActorFaceVelocityVector))

(event Input|AxisEvents|InputAxisRotateCamera(A/E)
  (params (AxisValue :type Float%20%28single-precision%29))
  ;[0.4531 0 1 0.5] Camera system
  ;;[0 1 0.08594 0.5] Camera Rotaion
  (Utilities|FlowControl|Gate true
    (:Exit
      (Pawn|Input|AddControllerYawInput AxisValue))))

(event Input|AxisEvents|InputAxisMoveForward/Backward(Z/S)
  (params (AxisValue :type Float%20%28single-precision%29))
  (bind _self self)
  (bind _returnvalue (Transformation|GetActorTransform _self))
  ;[1 0.9375 0 0.5] Mouvement
  ;;[0 0.0625 1] Movement CtoS
  (Variables|Default|SetPreMovementTransform (Transformation|GetActorTransform self))
  (Pawn|Input|AddMovementInput (Math|Vector|GetForwardVector (Math|Rotator|MakeRotator 0.0 0.0 (.yaw (Pawn|GetControlRotation self :!class /Script/Engine.Pawn)))) AxisValue false)
  ;;;[1 0.2812 0 0.5] AntiSpamServeur
  (if (not (== (Variables|Default|GetPreMovementTransform) (Transformation|GetActorTransform self)))
    (bind _aspc_main (Utilities|Casting|CastTopc_Main (Pawn|GetController)))
    (CallFunction|MoveCtoS _aspc_main (.location _returnvalue) (.rotation _returnvalue))))

(event Input|AxisEvents|InputAxisMoveLeft/Right(Q/D)
  (params (AxisValue :type Float%20%28single-precision%29))
  (bind _self self)
  (bind _returnvalue (Transformation|GetActorTransform _self))
  ;[1 0.9375 0 0.5] Mouvement
  ;;[0 0.0625 1] Movement CtoS
  (Pawn|Input|AddMovementInput (Math|Vector|GetRightVector (Math|Rotator|MakeRotator 0.0 0.0 (.yaw (Pawn|GetControlRotation self :!class /Script/Engine.Pawn)))) AxisValue false)
  ;;;[1 0.2812 0 0.5] AntiSpamServeur
  (if (not (== (Variables|Default|GetPreMovementTransform) (Transformation|GetActorTransform self)))
    (bind _aspc_main (Utilities|Casting|CastTopc_Main (Pawn|GetController)))
    (CallFunction|MoveCtoS _aspc_main (.location _returnvalue) (.rotation _returnvalue))))

(event Input|KeyboardEvents|LeftShift
  (params (Key :type Key%20Structure :default "None"))
  ;[0.4531 0 1 0.5] Camera system
  ;;[0 1 0.08594 0.5] Camera Rotaion
  (:Pressed
    (Utilities|FlowControl|Gate true) ; enters at Open
  )
  (:Released
    (Utilities|FlowControl|Gate true) ; enters at Close
  ))

(fn ConstructionScript
  (bind _asps_main (Utilities|Casting|CastTops_Main (Variables|GetPlayerState)))
  (Variables|/Game/Blueprints/Player/ps_Main.ps_Main_C|SetHero%20Struct _asps_main (Variables|Default|GetStats)))

(fn Gravity
  (bind _returnvalue (Transformation|GetActorLocation))
  (if (Variables|Default|GetIs%20Jumping)
    (Utilities|FlowControl|Sequence
      (:then_0
        (Variables|Default|SetTimePower (Math|Float|Clamp(Float) (+ (Variables|Default|GetTimePower) (* (Utilities|Time|GetWorldDeltaSeconds) (Variables|Default|GetAir%20Suspenstion%20Time))) 0.0 (Variables|Default|GetFalling%20Speed%20Max)))
        (Transformation|SetActorLocation (Math|Vector|MakeVector (.x _returnvalue) (.y _returnvalue) (- (.z _returnvalue) (* (Variables|Default|GetTimePower) (Variables|Default|GetGravity%20Power)))) true false)
        (return))
      (:then_1
        (Utilities|FlowControl|DoOnce false :!label _label
          (:Completed
            (goto _label_2 Reset)))))
    (else
      (Utilities|FlowControl|DoOnce false :!label _label_2
        (:Completed
          (Variables|Default|SetTimePower 0.0)
          (goto _label Reset))))))

(fn IsJumping?
  (bind _skeletalmesh (Variables|Default|GetSkeletalMesh))
  (bind _returnvalue (Transformation|GetWorldLocation _skeletalmesh))
  (bind _returnvalue_2 (Collision|LineTraceByChannel _returnvalue (- _returnvalue (* "0, 0,-1.000000" -1.3e+02)) "TraceTypeQuery1" false 0 "None"))
  (Variables|Default|SetIs%20Jumping (not _returnvalue_2))
  (return))