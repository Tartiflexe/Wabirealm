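; Main game mode that tracks connected player controllers and keeps the game state's name-to-controller list in sync.
; On login, each pc_Main joins a local array, has its player name suffixed with the resulting array index, and is registered in gs_Main under that name.
; On logout, the controller is removed from both the array and the game state list.
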(event EventOnLogout
  (params (ExitingController :type Controller%20Object%20Reference))
  ;[0.2656 1 0 0.5] Remove from Name/Controller list
  (bind _aspc_main (Utilities|Casting|CastTopc_Main ExitingController))
  (Utilities|Array|RemoveItem (Variables|Default|GetAllPlayersController) _aspc_main)
  (bind _asgs_main (Utilities|Casting|CastTogs_Main (Game|GetGameState)))
  (Default|RemovefromName/ControllerList _asgs_main _aspc_main))

(event EventPostLogin
  (params (NewPlayer :type Player%20Controller%20Object%20Reference))
  ;[0 0.4375 1 0.5] Name/Controller List
  (bind _aspc_main (Utilities|Casting|CastTopc_Main NewPlayer))
  (bind _returnvalue (Utilities|Array|Add (Variables|Default|GetAllPlayersController) _aspc_main))
  (Variables|/Game/Blueprints/Player/pc_Main.pc_Main_C|SetPlayerInfos _aspc_main (Utilities|Struct|Makes_PlayerInfos (Utilities|String|StringToName (Utilities|String|ToString(Text) (Utilities|Text|FormatText "{Name}_{nmbr}" (Utilities|Text|ToText(String) (Utilities|String|ToString(Name) (Utilities|Struct|Breaks_PlayerInfos (Variables|/Game/Blueprints/Player/pc_Main.pc_Main_C|GetPlayerInfos _aspc_main)))) _returnvalue)))))
  (bind _asgs_main (Utilities|Casting|CastTogs_Main (Game|GetGameState)))
  (Default|AddtoName/ControllerList _asgs_main (Utilities|String|StringToName (Utilities|String|ToString(Text) (Utilities|Text|FormatText "{Name}_{nmbr}" (Utilities|Text|ToText(String) (Utilities|String|ToString(Name) (Utilities|Struct|Breaks_PlayerInfos (Variables|/Game/Blueprints/Player/pc_Main.pc_Main_C|GetPlayerInfos _aspc_main)))) _returnvalue))) _aspc_main))

(fn ConstructionScript)