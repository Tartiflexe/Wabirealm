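; Main game state Blueprint, by its gs_ prefix, that serves as a registry for player controllers and stored player transforms.
; Events add controllers to the NameController map by name and remove them using the player name in their PlayerInfos.
; Another event stores player transforms in ControllerTransform, replacing any existing entry for the key.
; A disconnected debug loop prints that transform map, and the construction script is empty.
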(event Custom|Add%20to%20Name/Controller%20List
  (params (Key :type Name%20%28by%20ref%29) (Value :type Pc%20Main%20Object%20Reference%20%28by%20ref%29))
  (Utilities|Map|Add (Variables|Default|GetName/Controller) Key Value))

(event Custom|Stock%20player%20position
  (params (Key :type Pc%20Main%20Object%20Reference%20%28by%20ref%29) (Value :type Transform%20%28by%20ref%29))
  (bind _controller_transform (Variables|Default|GetController%20transform))
  ;[1 0 0.9844 0.5] Stock player transform
  (if (Utilities|Map|Contains _controller_transform Key)
    (Utilities|Map|Remove (Variables|Default|GetController%20transform) Key))
  (Utilities|Map|Add _controller_transform Key Value))

(event Custom|Remove%20from%20Name/Controller%20List
  (params (Value :type Pc%20Main%20Object%20Reference%20%28by%20ref%29))
  (Utilities|Map|Remove (Variables|Default|GetName/Controller) (Utilities|Struct|Breaks_PlayerInfos (Variables|/Game/Blueprints/Player/pc_Main.pc_Main_C|GetPlayerInfos Value))))

(fn ConstructionScript)