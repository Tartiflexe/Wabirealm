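; Game mode for the multiplayer lobby that tracks connected lobby player controllers and keeps the player count current.
; On post-login it adds the pc_Lobby to its controller list, waits briefly, then tells that controller to run its lobby HUD.
; Both login and logout update the list and pass its length to gs_Lobby through UpdatePlayers.
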(event EventBeginPlay)

(event EventTick
  (params (DeltaSeconds :type Float%20%28single-precision%29)))

(event EventPostLogin
  (params (NewPlayer :type Player%20Controller%20Object%20Reference))
  ;[0 0.9766 1 0.5] Login
  (bind _aspc_lobby (Utilities|Casting|CastTopc_Lobby NewPlayer))
  (Utilities|Array|Add (Variables|Default|GetAllPlayerController) _aspc_lobby)
  ;;[1 0 0.4922 0.5] Or to fast
  (Utilities|FlowControl|Delay 0.05)
  (Default|HudLobby _aspc_lobby)
  ;;[0.4766 0 1 0.5] Update Players
  (bind _asgs_lobby (Utilities|Casting|CastTogs_Lobby (Game|GetGameState)))
  (Default|UpdatePlayers _asgs_lobby (Utilities|Array|Length (Variables|Default|GetAllPlayerController))))

(event EventOnLogout
  (params (ExitingController :type Controller%20Object%20Reference))
  ;[0.7344 1 0 0.5] Logout
  (bind _aspc_lobby (Utilities|Casting|CastTopc_Lobby ExitingController))
  (Utilities|Array|RemoveItem (Variables|Default|GetAllPlayerController) _aspc_lobby)
  (bind _asgs_lobby (Utilities|Casting|CastTogs_Lobby (Game|GetGameState)))
  (Default|UpdatePlayers _asgs_lobby (Utilities|Array|Length (Variables|Default|GetAllPlayerController))))

(fn ConstructionScript)