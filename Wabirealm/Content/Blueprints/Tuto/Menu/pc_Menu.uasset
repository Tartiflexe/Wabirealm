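; Player controller for the main menu that handles hosting, finding and joining multiplayer sessions.
; On BeginPlay without authority, it creates the connection HUD and shows a locked cursor in Game and UI input mode.
; Hosting creates an online session and opens the lobby map as a listen server.
; Searching fills the HUD's session box with a widget per result, while joining uses a search result or an IP via the open console command.
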(event Custom|HUD%20-%20Menu
  ;[1 0.001249 0.5013] HUD-Menu
  (Utilities|IsValid (Variables|Default|GetHUD%20menu)
    (:Is%20Not%20Valid
      (bind _returnvalue (UserInterface|CreateWidget "/Game/Blueprints/Tuto/Menu/HUD/widget_ConnexionHud.widget_ConnexionHud_C"))
      (bind _output_get (Variables|Default|SetHUD%20menu _returnvalue))
      (UserInterface|Viewport|AddtoViewport _output_get 0))))

(event Custom|Init%20cursor
  ;[1 0.2812 0 0.5] Init Cursor
  (Variables|Default|SetbShowMouseCursor true)
  (Input|SetInputModeGameandUI self 0 "LockAlways" false))

(event Custom|Héberger
  ;[1 0.9375 0 0.5] Héberger
  (|Session self 5 false
    (:then
      (Game|OpenLevel(byName) "map_Lobby" true "listen"))))

(event Custom|Rejoindre
  (params (IP :type String))
  ;[0 0.9297 1 0.5] Rejoindre
  (Development|ExecuteConsoleCommand (Utilities|String|Append "open " IP) 0))

(event Custom|Rechercher
  ;[0.3828 0 1 0.5] Rechercher
  (Widget|Panel|ClearChildren (Variables|/Game/Blueprints/Tuto/Menu/HUD/widget_ConnexionHud.widget_ConnexionHud_C|GetSessionbox (Variables|Default|GetHUD%20menu)))
  (Variables|Default|SetIs%20findingSessions true)
  (bind _results (|FindSessions self 4 false)
    (:OnSuccess
      (for _array_element _results
        (bind _returnvalue (UserInterface|CreateWidget "/Game/Blueprints/Tuto/Menu/HUD/widget_sessions.widget_sessions_C" 0 _array_element))
        (Widget|Panel|AddChild (Variables|/Game/Blueprints/Tuto/Menu/HUD/widget_ConnexionHud.widget_ConnexionHud_C|GetSessionbox (Variables|Default|GetHUD%20menu)) _returnvalue))
      (Variables|Default|SetIs%20findingSessions false))))

(event Custom|Join%20session
  (params (SearchResult :type Blueprint%20Session%20Result%20Structure%20%28by%20ref%29))
  (|JoinSession self SearchResult))

(event EventBeginPlay
  ;[1 0.7636 0] Init
  (if (not (Ability|HasAuthority))
    (CallFunction|HUD-Menu)
    (CallFunction|InitCursor)))

(fn ConstructionScript)